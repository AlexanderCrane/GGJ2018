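; Satellite actor that holds the player in place on contact and lets them launch straight upward with E.
; Actor or box overlap with a Player-tagged actor disables character movement and sets IsLaunched on the ThirdPersonCharacter.
; With input enabled at BeginPlay, pressing E while that flag is set restores walking and launches the character, with a DoOnce and delay as launch cooldown.
; The flag is never cleared here.
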(event OnComponentBeginOverlap(Box)
  (params (OverlappedComponent :type Primitive%20Component%20Object%20Reference) (OtherActor :type Actor%20Object%20Reference) (OtherComp :type Primitive%20Component%20Object%20Reference) (OtherBodyIndex :type Integer) (bFromSweep :type Boolean) (SweepResult :type Hit%20Result%20Structure%20%28by%20ref%29))
  (if (Actor|ActorHasTag OtherActor "Player")
    (bind _asthird_person_character (Utilities|Casting|CastToThirdPersonCharacter (Game|GetPlayerCharacter 0)))
    (bind _output_get (Variables|Default|SetPlayerReference _asthird_person_character))
    (Pawn|Components|CharacterMovement|DisableMovement (Variables|/Script/Engine.Character|GetCharacterMovement _output_get))
    (bind _output_get_2 (Variables|/Game/ThirdPersonBP/Blueprints/ThirdPersonCharacter.ThirdPersonCharacter_C|SetisLaunched _asthird_person_character true))))

(event Collision|EventActorBeginOverlap
  (params (OtherActor :type Actor%20Object%20Reference))
  (if (Actor|ActorHasTag (stale OnComponentBeginOverlap(Box) OtherActor) "Player")
    (bind _asthird_person_character (Utilities|Casting|CastToThirdPersonCharacter (Game|GetPlayerCharacter 0)))
    (bind _output_get (Variables|Default|SetPlayerReference _asthird_person_character))
    (Pawn|Components|CharacterMovement|DisableMovement (Variables|/Script/Engine.Character|GetCharacterMovement _output_get))
    (bind _output_get_2 (Variables|/Game/ThirdPersonBP/Blueprints/ThirdPersonCharacter.ThirdPersonCharacter_C|SetisLaunched _asthird_person_character true))))

(event EventTick
  (params (DeltaSeconds :type Float%20%28single-precision%29)))

(event EventBeginPlay
  (Input|EnableInput (Game|GetPlayerController 0)))

(event Input|KeyboardEvents|E
  (params (Key :type Key%20Structure))
  (:Pressed
    (if (stale OnComponentBeginOverlap(Box) _output_get_2)
      (Pawn|Components|CharacterMovement|SetMovementMode (Variables|/Script/Engine.Character|GetCharacterMovement (stale OnComponentBeginOverlap(Box) _output_get)) "MOVE_Walking" 0)
      (Utilities|FlowControl|DoOnce false :!label _label
        (:Completed
          (Character|LaunchCharacter (stale OnComponentBeginOverlap(Box) _output_get) "0, 0,2000.000000" false false)
          (Utilities|FlowControl|Delay 3.0)
          (goto _label Reset))))))

(fn ConstructionScript)